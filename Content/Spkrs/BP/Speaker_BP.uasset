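; Speaker actor made of clickable meshes that forwards clicks by part group to a SpeakerLogic reference.
; Feet, frame and plate report as accents, woofers and horn tweeter as speaker components, while screen and cabinet report separately.
; InitializeSpeaker stores that reference and uses EnableCover to show or hide frame and screen, ignoring collision on them when hidden.
; Getter functions expose the meshes by group.
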(event `self.Foot_BL.OnClicked`
  (params (TouchedComponent :type "PrimitiveComponent Object Reference") (ButtonPressed :type "Key Structure"))
  ;[1 1 1] Accent Clicked
  (`/Game/Spkrs/BP/Speaker_Logic_BP.AccentsClicked` (`self.SpeakerLogic`) :!label _label))

(event `self.Foot_BR.OnClicked`
  (params (TouchedComponent :type "PrimitiveComponent Object Reference") (ButtonPressed :type "Key Structure"))
  ;[1 1 1] Accent Clicked
  (goto _label))

(event `self.Foot_FL.OnClicked`
  (params (TouchedComponent :type "PrimitiveComponent Object Reference") (ButtonPressed :type "Key Structure"))
  ;[1 1 1] Accent Clicked
  (goto _label))

(event `self.Foot_FR.OnClicked`
  (params (TouchedComponent :type "PrimitiveComponent Object Reference") (ButtonPressed :type "Key Structure"))
  ;[1 1 1] Accent Clicked
  (goto _label))

(event `self.AccentPlate.OnClicked`
  (params (TouchedComponent :type "PrimitiveComponent Object Reference") (ButtonPressed :type "Key Structure"))
  ;[1 1 1] Accent Clicked
  (goto _label))

(event `self.Frame.OnClicked`
  (params (TouchedComponent :type "PrimitiveComponent Object Reference") (ButtonPressed :type "Key Structure"))
  ;[1 1 1] Accent Clicked
  (goto _label))

(event `self.Woofers.OnClicked`
  (params (TouchedComponent :type "PrimitiveComponent Object Reference") (ButtonPressed :type "Key Structure"))
  ;[1 1 1] Speakers Clicked
  (`/Game/Spkrs/BP/Speaker_Logic_BP.SpeakerComponentsClicked` (`self.SpeakerLogic`) :!label _label_2))

(event `self.HornTweeter.OnClicked`
  (params (TouchedComponent :type "PrimitiveComponent Object Reference") (ButtonPressed :type "Key Structure"))
  ;[1 1 1] Speakers Clicked
  (goto _label_2))

(event `self.Screen.OnClicked`
  (params (TouchedComponent :type "PrimitiveComponent Object Reference") (ButtonPressed :type "Key Structure"))
  ;[1 1 1] Screen Clicked
  (`/Game/Spkrs/BP/Speaker_Logic_BP.ScreenClicked` (`self.SpeakerLogic`)))

(event `self.Cabinette.OnClicked`
  (params (TouchedComponent :type "PrimitiveComponent Object Reference") (ButtonPressed :type "Key Structure"))
  ;[1 1 1] Cabinet Clicked
  (`/Game/Spkrs/BP/Speaker_Logic_BP.CabinetClicked` (`self.SpeakerLogic`)))

(fn `GetAccentsMeshes`
  (returns (FootMeshes :type "Array of MeshComponent Object Reference") (AccentMeshes :type "Array of MeshComponent Object Reference"))
  (return (`|MakeArray` (`self.Foot_BR`) (`self.Foot_FL`) (`self.Foot_FR`) (`self.Foot_BL`) :!type "MeshComponent Object Reference") (`|MakeArray` (`self.Frame`) (`self.AccentPlate`) :!type "MeshComponent Object Reference")))

(fn `GetCabinetComponent`
  (returns (MeshComponent :type "MeshComponent Object Reference"))
  (return (`self.Cabinette`)))

(fn `GetScreenMesh`
  (returns (ScreenMesh :type "MeshComponent Object Reference"))
  (return (`self.Screen`)))

(fn `GetSpeakerComponents`
  (returns (TweeterMesh :type "MeshComponent Object Reference") (WoofersMesh :type "MeshComponent Object Reference"))
  (return (`self.HornTweeter`) (`self.Woofers`)))

(fn `InitializeSpeaker`
  (params (SpeakerLogic :type "/Game/Spkrs/BP/Speaker_Logic_BP Object Reference"))
  (`|ExecutionSequence`
    (:`then_0`
      (set `self.SpeakerLogic` SpeakerLogic))
    (:`then_1`
      ;[1 1 1] Enable or Disable Cover
      (if (`self.Enable Cover`)
        ;;[0 1 0] Enable Cover
        (`SceneComponent.SetVisibility` (`self.Frame`) true false)
        (`SceneComponent.SetVisibility` (`self.Screen`) true false)
        (else
          ;;[1 0 0] Disable Cover
          (`SceneComponent.SetVisibility` (`self.Frame`) false false)
          (`SceneComponent.SetVisibility` (`self.Screen`) false false)
          (`PrimitiveComponent.SetCollisionResponseToAllChannels` (`self.Frame`) "ECR_Ignore")
          (`PrimitiveComponent.SetCollisionResponseToAllChannels` (`self.Screen`) "ECR_Ignore"))))))

(fn `UserConstructionScript`)