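; Speaker configurator logic that cycles finishes on a list of speakers and shows the resulting options and cost on the HUD.
; Click functions step wrapping indices for cabinet, drivers, accents and screen, then apply materials or a screen color parameter to every speaker.
; Each index also keys a data table row whose descriptions and cent-based prices feed the HUD summary and USD total.
; A separate function switches music tracks on an audio component.
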(fn `AccentsClicked`
  (bind _output_get (set `self.AccentIndex` (mod (+ (`self.AccentIndex`) 1) (`self.AccentIndexMax`))))
  (switch `int` _output_get
    (:`0`
      (`self.SetAccentMaterial` "/Game/Spkrs/m/BlkGld_Ft.BlkGld_Ft" "/Game/Spkrs/m/BlkGld_Cab.BlkGld_Cab"))
    (:`1`
      (`self.SetAccentMaterial` "/Game/Spkrs/m/EbStl_Ft.EbStl_Ft" "/Game/Spkrs/m/EbStl_Cab.EbStl_Cab"))
    (:`2`
      (`self.SetAccentMaterial` "/Game/Spkrs/m/TkBlk_Ft.TkBlk_Ft" "/Game/Spkrs/m/TkBlk_Cab.TkBlk_Cab"))
    (:`3`
      (`self.SetAccentMaterial` "/Game/Spkrs/m/WalSlv_Ft.WalSlv_Ft" "/Game/Spkrs/m/WalSlv_Cab.WalSlv_Cab"))
    (:`4`
      (`self.SetAccentMaterial` "/Game/Spkrs/m/WhtCp_Ft.WhtCp_Ft" "/Game/Spkrs/m/WhtCp_Cab.WhtCp_Cab")))
  (`self.DisplayAccentData` (`self.AccentIndex`)))

(fn `CabinetClicked`
  (bind _output_get (set `self.CabinetIndex` (mod (+ (`self.CabinetIndex`) 1) (`self.CabinetIndexMax`))))
  (switch `int` _output_get
    (:`0`
      (`self.SetCabinetMaterial` "/Game/Spkrs/m/BlkGld_Cab.BlkGld_Cab"))
    (:`1`
      (`self.SetCabinetMaterial` "/Game/Spkrs/m/EbStl_Cab.EbStl_Cab"))
    (:`2`
      (`self.SetCabinetMaterial` "/Game/Spkrs/m/TkBlk_Cab.TkBlk_Cab"))
    (:`3`
      (`self.SetCabinetMaterial` "/Game/Spkrs/m/WalSlv_Cab.WalSlv_Cab"))
    (:`4`
      (`self.SetCabinetMaterial` "/Game/Spkrs/m/WhtCp_Cab.WhtCp_Cab")))
  (`self.DisplayCabinetData` (`self.CabinetIndex`)))

(fn `Display Final Data to Hud`
  (`|ExecutionSequence`
    (:`then_0`
      ;[1 1 1] Set Total Prices
      (set `/Game/HUD/HUD_UI.TotalPrice` (`self.FormatPrice` (+ (`self.BasePrice`) (`self.CabinetPrice`) (`self.SpeakerPrice`) (`self.AccentPrice`) (`self.ScreenPrice`))) (`self.HUD`)))
    (:`then_1`
      ;[1 1 1] Set Prices
      (set `/Game/HUD/HUD_UI.BasePrice` (`self.FormatPrice` (`self.BasePrice`)) (`self.HUD`))
      (set `/Game/HUD/HUD_UI.CabinetPrice` (`self.FormatPrice` (`self.CabinetPrice`)) (`self.HUD`))
      (set `/Game/HUD/HUD_UI.SpeakerPrice` (`self.FormatPrice` (`self.SpeakerPrice`)) (`self.HUD`))
      (set `/Game/HUD/HUD_UI.AccentPrice` (`self.FormatPrice` (`self.AccentPrice`)) (`self.HUD`))
      (set `/Game/HUD/HUD_UI.ScreenPrice` (`self.FormatPrice` (`self.ScreenPrice`)) (`self.HUD`)))
    (:`then_2`
      ;[1 1 1] Set Short Description
      (set `/Game/HUD/HUD_UI.CabinetChoice` (`self.CabinetShortDescription`) (`self.HUD`))
      (set `/Game/HUD/HUD_UI.SpeakerChoice` (`self.SpeakerShortDescription`) (`self.HUD`))
      (set `/Game/HUD/HUD_UI.AccentChoice` (`self.AccentShortDescription`) (`self.HUD`))
      (set `/Game/HUD/HUD_UI.ScreenChoice` (`self.ScreenShortDescription`) (`self.HUD`)))
    (:`then_3`
      ;[1 1 1] Set Description
      (set `/Game/HUD/HUD_UI.Description` (`KismetTextLibrary.Conv_StringToText` (`KismetStringLibrary.Concat_StrStr` (`KismetTextLibrary.Conv_TextToString` (`self.SpeakerLongDescription`)) " Mounted in " (`KismetTextLibrary.Conv_TextToString` (`self.CabinetLongDescription`)) " Cabinets and " (`KismetTextLibrary.Conv_TextToString` (`self.AccentLongDescription`)))) (`self.HUD`)))))

(fn `DisplayAccentData`
  (params (Index :type Integer))
  (bind _returnvalue (`|GetDataTableRow` "/Game/Data/Accent_Data.Accent_Data" (`KismetStringLibrary.Conv_StringToName` (`KismetStringLibrary.Conv_IntToString` Index)))
    (:`then`
      (`|ExecutionSequence`
        (:`then_0`
          (bind (_shortdescription _longdescription _price) (break `/Game/Data/SpeakerData_Structure` _returnvalue))
          (set `self.AccentShortDescription` _shortdescription))
        (:`then_1`
          (set `self.AccentLongDescription` _longdescription))
        (:`then_2`
          (set `self.AccentPrice` _price))
        (:`then_3`
          (`self.Display Final Data to Hud`))))))

(fn `DisplayCabinetData`
  (params (Index :type Integer))
  (bind _returnvalue (`|GetDataTableRow` "/Game/Data/Cabinette_Data.Cabinette_Data" (`KismetStringLibrary.Conv_StringToName` (`KismetStringLibrary.Conv_IntToString` Index)))
    (:`then`
      (`|ExecutionSequence`
        (:`then_0`
          (bind (_shortdescription _longdescription _price) (break `/Game/Data/SpeakerData_Structure` _returnvalue))
          (set `self.CabinetShortDescription` _shortdescription))
        (:`then_1`
          (set `self.CabinetLongDescription` _longdescription))
        (:`then_2`
          (set `self.CabinetPrice` _price))
        (:`then_3`
          (`self.Display Final Data to Hud`))))))

(fn `DisplayScreenData`
  (params (Index :type Integer))
  (bind _returnvalue (`|GetDataTableRow` "/Game/Data/Screen_Data.Screen_Data" (`KismetStringLibrary.Conv_StringToName` (`KismetStringLibrary.Conv_IntToString` Index)))
    (:`then`
      (`|ExecutionSequence`
        (:`then_0`
          (bind (_shortdescription _longdescription _price) (break `/Game/Data/SpeakerData_Structure` _returnvalue))
          (set `self.ScreenShortDescription` _shortdescription))
        (:`then_1`
          (set `self.ScreenPrice` _price))
        (:`then_2`
          (`self.Display Final Data to Hud`))))))

(fn `DisplaySpeakerData`
  (params (Index :type Integer))
  (bind _returnvalue (`|GetDataTableRow` "/Game/Data/Speaker_Data.Speaker_Data" (`KismetStringLibrary.Conv_StringToName` (`KismetStringLibrary.Conv_IntToString` Index)))
    (:`then`
      (`|ExecutionSequence`
        (:`then_0`
          (bind (_shortdescription _longdescription _price) (break `/Game/Data/SpeakerData_Structure` _returnvalue))
          (set `self.SpeakerShortDescription` _shortdescription))
        (:`then_1`
          (set `self.SpeakerLongDescription` _longdescription))
        (:`then_2`
          (set `self.SpeakerPrice` _price))
        (:`then_3`
          (`self.Display Final Data to Hud`))))))

(fn `FormatPrice`
  (params (PriceInCents :type Integer))
  (returns (FormattedPrice :type Text))
  (return (`KismetTextLibrary.AsCurrencyBase` PriceInCents "USD")))

(fn `InitializeSpeakerLogic`
  (params (SpeakerList :type "Array of /Game/Spkrs/BP/Speaker_BP Object Reference") (HUD :type "/Game/HUD/HUD_UI Object Reference"))
  (`|ExecutionSequence`
    (:`then_0`
      (set `self.SpeakerList` SpeakerList))
    (:`then_1`
      (set `self.HUD` HUD))
    (:`then_2`
      ;[1 1 1] Initialize HUD Data
      (`self.DisplayCabinetData` 0)
      (`self.DisplaySpeakerData` 0)
      (`self.DisplayAccentData` 0)
      (`self.DisplayScreenData` 0))))

(fn `PlayAudio`
  (params (TrackIndex :type Integer))
  (`|ExecutionSequence`
    (:`then_0`
      ;[1 1 1] Stop Audio Component
      (`AudioComponent.Stop` (`self.AudioComponent`)))
    (:`then_1`
      ;[1 1 1] Set Sound Track
      (`AudioComponent.SetSound` (`self.AudioComponent`) (`|GetArrayItem` (`self.MusicTracks`) TrackIndex)))
    (:`then_2`
      ;[1 1 1] Play Audio Component
      (`AudioComponent.Play` (`self.AudioComponent`) 0.0))))

(fn `ScreenClicked`
  (bind _output_get (set `self.ScreenIndex` (mod (+ (`self.ScreenIndex`) 1) (`self.ScreenIndexMax`))))
  (switch `int` _output_get
    (:`0`
      ;[1 1 1] Black
      (`self.SetScreenColor` (0.0 0.0 0.0)))
    (:`1`
      ;[1 1 1] Gold
      (`self.SetScreenColor` (0.1441 0.1155 0.0323)))
    (:`2`
      ;[1 1 1] Dark Grey
      (`self.SetScreenColor` (0.089 0.089 0.089)))
    (:`3`
      ;[1 1 1] White
      (`self.SetScreenColor` (1.0 1.0 1.0)))
    (:`4`
      ;[1 1 1] Dark Brown
      (`self.SetScreenColor` (0.0642 0.0237 0.0093))))
  (`self.DisplayScreenData` (`self.ScreenIndex`)))

(fn `SetAccentMaterial`
  (params (FootMaterial :type "Material Object Reference") (AccentMaterial :type "Material Object Reference"))
  (for _array_element (`self.SpeakerList`)
    (bind (_footmeshes _accentmeshes) (`/Game/Spkrs/BP/Speaker_BP.GetAccentsMeshes` _array_element))
    (`|ExecutionSequence`
      (:`then_0`
        (for _array_element_2 _footmeshes
          (`PrimitiveComponent.SetMaterial` _array_element_2 0 FootMaterial)))
      (:`then_1`
        (for _array_element_3 _accentmeshes
          (`PrimitiveComponent.SetMaterial` _array_element_3 0 AccentMaterial))))))

(fn `SetCabinetMaterial`
  (params (Material :type "Material Object Reference"))
  (for _array_element (`self.SpeakerList`)
    (bind _meshcomponent (`/Game/Spkrs/BP/Speaker_BP.GetCabinetComponent` _array_element))
    (`PrimitiveComponent.SetMaterial` _meshcomponent 0 Material)))

(fn `SetScreenColor`
  (params (Color :type "Vector Structure"))
  (for _array_element (`self.SpeakerList`)
    (bind _screenmesh (`/Game/Spkrs/BP/Speaker_BP.GetScreenMesh` _array_element))
    (`MeshComponent.SetVectorParameterValueOnMaterials` _screenmesh "Color" Color)))

(fn `SetSpeakerComponentsMaterial`
  (params (TweeterMaterial :type "Material Object Reference") (WoofersMaterial :type "Material Object Reference"))
  (for _array_element (`self.SpeakerList`)
    (bind (_tweetermesh _woofersmesh) (`/Game/Spkrs/BP/Speaker_BP.GetSpeakerComponents` _array_element))
    (`|ExecutionSequence`
      (:`then_0`
        (`PrimitiveComponent.SetMaterial` _tweetermesh 0 TweeterMaterial))
      (:`then_1`
        (`PrimitiveComponent.SetMaterial` _woofersmesh 0 WoofersMaterial)))))

(fn `SpeakerComponentsClicked`
  (bind _output_get (set `self.SpeakerComponentIndex` (mod (+ (`self.SpeakerComponentIndex`) 1) (`self.SpeakerComponentMax`))))
  (switch `int` _output_get
    (:`0`
      (`self.SetSpeakerComponentsMaterial` "/Game/Spkrs/m/TkBlk_Twt.TkBlk_Twt" "/Game/Spkrs/m/TkBlk_Wof.TkBlk_Wof"))
    (:`1`
      (`self.SetSpeakerComponentsMaterial` "/Game/Spkrs/m/BlkGld_Twt.BlkGld_Twt" "/Game/Spkrs/m/BlkGld_Wof.BlkGld_Wof"))
    (:`2`
      (`self.SetSpeakerComponentsMaterial` "/Game/Spkrs/m/WalSlv_Twt.WalSlv_Twt" "/Game/Spkrs/m/WalSlv_Wof.WalSlv_Wof"))
    (:`3`
      (`self.SetSpeakerComponentsMaterial` "/Game/Spkrs/m/WhtCp_Twt.WhtCp_Twt" "/Game/Spkrs/m/WhtCp_Wof.WhtCp_Wof")))
  (`self.DisplaySpeakerData` (`self.SpeakerComponentIndex`)))

(fn `UserConstructionScript`)